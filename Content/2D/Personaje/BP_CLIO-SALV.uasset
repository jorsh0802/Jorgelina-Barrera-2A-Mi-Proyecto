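; Player character CLIO for a side-scrolling game, with Enhanced Input for movement along X, jumping and quitting.
; Acceleration direction flips control yaw to face left or right.
; Landing, jumping and leaving ledges set double-jump and coyote-time flags, timed by retriggerable delays, though nothing here reads them.
; Health, healing and coin events update totals with on-screen debug messages; health is never clamped.
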(event Input|EnhancedActionEvents|EnhancedInputActionIA_SalirJuego
  (params (ActionValue :type Float%20%28double-precision%29) (ElapsedSeconds :type Float%20%28double-precision%29) (TriggeredSeconds :type Float%20%28double-precision%29) (InputAction :type Input%20Action%20Object%20Reference :default "/Game/2D/Personaje/INPUTS/IA_SalirJuego.IA_SalirJuego"))
  (:Started
    (Game|QuitGame 0 "Quit" false)))

(event Input|EnhancedActionEvents|EnhancedInputActionIA_Movimiento
  (params (ActionValue :type Float%20%28double-precision%29) (ElapsedSeconds :type Float%20%28double-precision%29) (TriggeredSeconds :type Float%20%28double-precision%29) (InputAction :type Input%20Action%20Object%20Reference :default "/Game/2D/Personaje/INPUTS/IA_Movimiento.IA_Movimiento"))
  (bind _returnvalue (Pawn|GetController))
  (Pawn|Input|AddMovementInput "1.000000,0.000000,0.000000" ActionValue false)
  (Math|Float|CompareFloat (.x (Pawn|Components|CharacterMovement|GetCurrentAcceleration (Variables|Character|GetCharacterMovement))) 0.0
    (:>
      (Pawn|SetControlRotation _returnvalue (Math|Rotator|MakeRotator 0.0 0.0 0.0)))
    (:<
      (Pawn|SetControlRotation _returnvalue (Math|Rotator|MakeRotator 0.0 0.0 1.8e+02)))))

(event Input|EnhancedActionEvents|EnhancedInputActionIA_Salto
  (params (ActionValue :type Float%20%28double-precision%29) (ElapsedSeconds :type Float%20%28double-precision%29) (TriggeredSeconds :type Float%20%28double-precision%29) (InputAction :type Input%20Action%20Object%20Reference :default "/Game/2D/Personaje/INPUTS/IA_Salto.IA_Salto"))
  (:Started
    (Character|Jump))
  (:Completed
    (Character|StopJumping)))

(event EventBeginPlay
  (bind _asplayer_controller (Utilities|Casting|CastToPlayerController (Pawn|GetController)))
  (Input|AddMappingContext (PlayerController|LocalPlayerSubsystems|GetEnhancedInputLocalPlayerSubsystem _asplayer_controller) "/Game/2D/Personaje/INPUTS/MAPPING/IMC_CLIO.IMC_CLIO" 0 "(bIgnoreAllPressedKeysUntilRelease=True,bForceImmediately=False,bNotifyUserSettings=False)"))

(event EventOnJumped
  (Variables|Default|SetDisponible%20Doble%20Salto true)
  (Utilities|FlowControl|RetriggerableDelay (Variables|Default|GetTiempo%20de%20Doble%20Salto))
  (Variables|Default|SetDisponible%20Doble%20Salto false))

(event EventOnWalkingOffLedge
  (params (PreviousFloorImpactNormal :type Vector%20%28by%20ref%29 :default "0, 0, 0") (PreviousFloorContactNormal :type Vector%20%28by%20ref%29 :default "0, 0, 0") (PreviousLocation :type Vector%20%28by%20ref%29 :default "0, 0, 0") (TimeDelta :type Float%20%28single-precision%29))
  (Variables|Default|SetEsta%20con%20Coyote%20Time true)
  (Utilities|FlowControl|RetriggerableDelay (Variables|Default|GetTiempo%20Coyote))
  (Variables|Default|SetEsta%20con%20Coyote%20Time false))

(event EventOnLanded
  (params (Hit :type Hit%20Result%20Structure%20%28by%20ref%29))
  (Variables|Default|SetPrimer%20Salto false)
  (Variables|Default|SetPuedo%20Saltar? true))

(event EventRestarHP
  (params (Restar%20Vida :type Float%20%28double-precision%29))
  (bind _output_get (Variables|Default|SetVida (+ Restar%20Vida (Variables|Default|GetVida))))
  (if (>= _output_get 0.0)
    (Development|PrintString (Utilities|String|Append "Tu Personaje esta 
sufriendo Daño : " (Utilities|String|ToString(Float) _output_get)) true true "(R=1.000000,G=0.412919,B=0.000000,A=1.000000)" 5.0)
    (else
      (Development|PrintString "Vida Acabada" true true "(R=1.000000,G=0.000000,B=0.052170,A=1.000000)"))))

(event EventCurar
  (params (Reg%20HP :type Float%20%28double-precision%29))
  (bind _output_get (Variables|Default|SetVida (+ Reg%20HP (Variables|Default|GetVida))))
  (if (<= _output_get 1e+02)
    (Development|PrintString (Utilities|String|Append "Tu Personaje se 
esta curando : " (Utilities|String|ToString(Float) _output_get)) true true "(R=0.000000,G=1.000000,B=0.581677,A=1.000000)" 5.0)
    (else
      (Variables|Default|SetVida%20Maxima (Variables|Default|GetVida%20Maxima))
      (if true
        (Development|PrintString "Vida Curado" true true "(R=0.259400,G=1.000000,B=0.000000,A=1.000000)")))))

(event EventObtenerMoneda
  (params (Monedas :type Integer))
  (bind _output_get (Variables|Default|SetMoneda (+ Monedas (Variables|Default|GetMoneda))))
  (Development|PrintString (Utilities|String|Append "Agarraste una Moneda. 
Tus Monedas Actuales son : " (Utilities|String|ToString(Integer) _output_get)) true true "(R=0.000000,G=0.569925,B=1.000000,A=1.000000)" 5.0))

(fn ConstructionScript)